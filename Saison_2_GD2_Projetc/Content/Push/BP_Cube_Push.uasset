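; Pushable cube that the third-person character can slide in four directions while interacting with it.
; The Forward trigger flags when interaction is allowed, and a Sphere overlap shows or hides a widget.
; Each Tick, the character's movement axes choose direction and speed for SpeedDirection, which nudges SMCube along its right or forward vector using VInterpTo, without sweep.
; Overlaps do not filter the overlapping actor, and debug prints report state.
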(event `self.ReceiveBeginPlay`
  (bind _returnvalue (`GameplayStatics.GetActorOfClass` "/Game/ThirdPerson/Blueprints/BP_ThirdPersonCharacter.BP_ThirdPersonCharacter_C"))
  (set `self.CharREF` _returnvalue))

(event `self.ReceiveTick`
  (params (DeltaSeconds :type "Float (single-precision)"))
  (bind _charref (`self.CharREF`))
  (bind _charref_2 (`self.CharREF`))
  (bind _forward_backward_axis (`/Game/ThirdPerson/Blueprints/BP_ThirdPersonCharacter.Forward Backward Axis` _charref))
  (bind _right_left_axis (`/Game/ThirdPerson/Blueprints/BP_ThirdPersonCharacter.Right Left Axis` _charref))
  (if (and (`/Game/ThirdPerson/Blueprints/BP_ThirdPersonCharacter.IsInteractingBox?` _charref_2) (`/Game/ThirdPerson/Blueprints/BP_ThirdPersonCharacter.CanIntecratcBox?` _charref_2) (`self.PlayerInFrontOf`))
    (`|ExecutionSequence`
      (:`then_0`
        (if (== _forward_backward_axis 0.0)
          (`KismetSystemLibrary.PrintString` "Is not moving Fwd or Bwd" true true (struct :`R` 1.0 :`B` 0.019788 :`A` 1.0) 2.0 "25427")
          (elif (>= _forward_backward_axis 0.1)
            (`KismetSystemLibrary.PrintString` "Is moving Forward" true true (struct :`G` 1.0 :`B` 0.098257 :`A` 1.0) 2.0 "526897378")
            (`self.Speed / Direction` true -25.0)
            (else
              (`KismetSystemLibrary.PrintString` "Is moving Backward" true true (struct :`G` 1.0 :`B` 0.098257 :`A` 1.0) 2.0 "5758778")
              (`self.Speed / Direction` true 25.0)))))
      (:`then_1`
        (if (== _right_left_axis 0.0)
          (`KismetSystemLibrary.PrintString` "Is not moving Fwd or Bwd" true true (struct :`R` 1.0 :`B` 0.019788 :`A` 1.0) 2.0 "25427")
          (elif (>= _right_left_axis 0.1)
            (`KismetSystemLibrary.PrintString` "Is moving Right" true true (struct :`G` 1.0 :`B` 0.098257 :`A` 1.0) 2.0 "526897378")
            (`self.Speed / Direction` false 27.5)
            (else
              (`KismetSystemLibrary.PrintString` "Is moving Left" true true (struct :`G` 1.0 :`B` 0.098257 :`A` 1.0) 2.0 "5758778")
              (`self.Speed / Direction` false -27.5))))))))

(event `self.Forward.OnComponentBeginOverlap`
  (params (OverlappedComponent :type "PrimitiveComponent Object Reference") (OtherActor :type "Actor Object Reference") (OtherComp :type "PrimitiveComponent Object Reference") (OtherBodyIndex :type Integer) (bFromSweep :type Boolean) (SweepResult :type "HitResult Structure (by ref)"))
  (`KismetSystemLibrary.PrintString` "Character can interact" true true (struct :`G` 1.0 :`B` 0.050582 :`A` 1.0) 2.0 "23565156")
  (set `/Game/ThirdPerson/Blueprints/BP_ThirdPersonCharacter.CanIntecratcBox?` true (`self.CharREF`))
  (set `self.PlayerInFrontOf` true))

(event `self.Forward.OnComponentEndOverlap`
  (params (OverlappedComponent :type "PrimitiveComponent Object Reference") (OtherActor :type "Actor Object Reference") (OtherComp :type "PrimitiveComponent Object Reference") (OtherBodyIndex :type Integer))
  (`KismetSystemLibrary.PrintString` "Character cannot interact" true true (struct :`R` 1.0 :`G` 0.027806 :`A` 1.0) 2.0 "24341424")
  (set `/Game/ThirdPerson/Blueprints/BP_ThirdPersonCharacter.CanIntecratcBox?` false (`self.CharREF`))
  (set `self.PlayerInFrontOf` false))

(event `self.Sphere.OnComponentBeginOverlap`
  (params (OverlappedComponent :type "PrimitiveComponent Object Reference") (OtherActor :type "Actor Object Reference") (OtherComp :type "PrimitiveComponent Object Reference") (OtherBodyIndex :type Integer) (bFromSweep :type Boolean) (SweepResult :type "HitResult Structure (by ref)"))
  (`SceneComponent.SetVisibility` (`self.Widget`) true false))

(event `self.Sphere.OnComponentEndOverlap`
  (params (OverlappedComponent :type "PrimitiveComponent Object Reference") (OtherActor :type "Actor Object Reference") (OtherComp :type "PrimitiveComponent Object Reference") (OtherBodyIndex :type Integer))
  (`SceneComponent.SetVisibility` (`self.Widget`) false false))

(fn `UserConstructionScript`)