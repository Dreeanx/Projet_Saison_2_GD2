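; Wall actor that moves vertically when triggered by its paired pressure plate, BP_Plaque_de_pression_Wall_6.
; On BeginPlay it finds the plate with GetActorOfClass and binds Open and Close to the plate's events.
; Separate timelines play forward to open and reverse to close, setting the mesh's absolute world Z while keeping X and Y, despite the track being named DoorRotation.
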(event `self.ReceiveBeginPlay`
  (bind _returnvalue (`GameplayStatics.GetActorOfClass` "/Game/Pressure_Plate/BP_Plaque_de_pression_Wall_6.BP_Plaque_de_pression_Wall_6_C"))
  (bind _output_get (set `self.Button 2 ref` _returnvalue))
  (add `/Game/Pressure_Plate/BP_Plaque_de_pression_Wall_6.Open 2` _output_get (delegate `open`))
  (add `/Game/Pressure_Plate/BP_Plaque_de_pression_Wall_6.Close 2` _output_get (delegate `close`)))

(event `open`
  (bind _staticmeshcomponent (`self.StaticMeshComponent`))
  (bind (_returnvalue_x _returnvalue_y) (`KismetMathLibrary.BreakVector` (`SceneComponent.K2_GetComponentLocation` _staticmeshcomponent)))
  (bind (_direction _door_rotation) (`Timeline|Timeline` :!via `PlayFromStart`)
    (:`Update`
      (`SceneComponent.K2_SetWorldLocation` _staticmeshcomponent (`KismetMathLibrary.MakeVector` _returnvalue_x _returnvalue_y _door_rotation) false false))))

(event `close`
  (bind _staticmeshcomponent (`self.StaticMeshComponent`))
  (bind (_returnvalue_x _returnvalue_y) (`KismetMathLibrary.BreakVector` (`SceneComponent.K2_GetComponentLocation` _staticmeshcomponent)))
  (bind (_direction _door_rotation) (`Timeline|Timeline_0` :!via `ReverseFromEnd`)
    (:`Update`
      (`SceneComponent.K2_SetWorldLocation` _staticmeshcomponent (`KismetMathLibrary.MakeVector` _returnvalue_x _returnvalue_y _door_rotation) false false))))

(fn `UserConstructionScript`)