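; Wall actor that rises and lowers in response to a pressure plate.
; On BeginPlay it finds a BP_Plaque_de_pression_Wall via GetActorOfClass and binds its open and close events to that plate.
; Each event plays its own timeline, whose curve drives a lerp from the mesh's current location toward a small vertical offset, up or down.
; Movement therefore accumulates every update rather than interpolating between fixed endpoints.
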(event `self.ReceiveBeginPlay`
  (bind _returnvalue (`GameplayStatics.GetActorOfClass` "/Game/Pressure_Plate/BP_Plaque_de_pression_Wall.BP_Plaque_de_pression_Wall_C"))
  (bind _output_get (set `self.Button Ref` _returnvalue))
  (add `/Game/Pressure_Plate/BP_Plaque_de_pression_Wall.Open` _output_get (delegate `open`))
  (add `/Game/Pressure_Plate/BP_Plaque_de_pression_Wall.Close` _returnvalue (delegate `close`)))

(event `open`
  (bind _returnvalue (`SceneComponent.K2_GetComponentLocation` (`self.StaticMeshComponent`)))
  (bind (_direction _door_rotation) (`Timeline|Timeline`)
    (:`Update`
      (`SceneComponent.K2_SetWorldLocation` (`self.StaticMeshComponent`) (`KismetMathLibrary.VLerp` _returnvalue (+ _returnvalue (0.0 0.0 10.0)) _door_rotation) false false))))

(event `close`
  (bind _returnvalue (`SceneComponent.K2_GetComponentLocation` (`self.StaticMeshComponent`)))
  (bind (_direction _door_rotation) (`Timeline|Timeline_0`)
    (:`Update`
      (`SceneComponent.K2_SetWorldLocation` (`self.StaticMeshComponent`) (`KismetMathLibrary.VLerp` _returnvalue (+ _returnvalue (0.0 0.0 -10.0)) _door_rotation) false false))))

(fn `UserConstructionScript`)