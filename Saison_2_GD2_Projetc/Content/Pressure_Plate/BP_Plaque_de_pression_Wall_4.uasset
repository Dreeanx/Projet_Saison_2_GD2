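; Pressure plate actor, named for Wall 4, that signals open and close as the player steps on and off it.
; On BeginPlay it adds the first player character to a list of accepted actors.
; Sphere overlap begin and end check the other actor against that list, calling Open1 on entry and Close1 on exit.
; What opens or closes is handled outside this graph.
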(event `self.ReceiveBeginPlay`
  (`KismetArrayLibrary.Array_Add` (`self.List`) (`GameplayStatics.GetPlayerCharacter` 0)))

(event `self.Sphere.OnComponentBeginOverlap`
  (params (OverlappedComponent :type "PrimitiveComponent Object Reference") (OtherActor :type "Actor Object Reference") (OtherComp :type "PrimitiveComponent Object Reference") (OtherBodyIndex :type Integer) (bFromSweep :type Boolean) (SweepResult :type "HitResult Structure (by ref)"))
  (for _array_element (`self.List`)
    (if (== _array_element OtherActor)
      (`self.Open 1`))))

(event `self.Sphere.OnComponentEndOverlap`
  (params (OverlappedComponent :type "PrimitiveComponent Object Reference") (OtherActor :type "Actor Object Reference") (OtherComp :type "PrimitiveComponent Object Reference") (OtherBodyIndex :type Integer))
  (for _array_element (`self.List`)
    (if (== _array_element OtherActor)
      (`self.Close 1`))))

(fn `UserConstructionScript`)