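; BP_Gate is a level-exit gate that opens once enough items are collected and sends the player to Level1_Spiritual.
; CollectItem counts pickups and, at the maximum, calls OpenDoor once after a delay.
; OpenDoor runs a timeline that lowers the Uwu component, lerping from its current location each update, so movement accumulates.
; Third-person character overlap with Trigger plays a sound and fade widget, then loads the level, independent of door state.
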(event `self.Trigger.OnComponentBeginOverlap`
  (params (OverlappedComponent :type "PrimitiveComponent Object Reference") (OtherActor :type "Actor Object Reference") (OtherComp :type "PrimitiveComponent Object Reference") (OtherBodyIndex :type Integer) (bFromSweep :type Boolean) (SweepResult :type "HitResult Structure (by ref)"))
  (cast `/Game/ThirdPerson/Blueprints/BP_ThirdPersonCharacter` OtherActor)
  (`GameplayStatics.PlaySound2D` null 1.0 1.0 0.0 null null)
  (bind _returnvalue (`|CreateWidget` "/Game/Travel_To_Next_Level/BP_Fade.BP_Fade_C"))
  (`UserWidget.AddToViewport` _returnvalue 0)
  (`/Game/Travel_To_Next_Level/BP_Fade.Fade_Anim` _returnvalue)
  (`KismetSystemLibrary.Delay` 0.5)
  (`GameplayStatics.OpenLevelBySoftObjectPtr` "/Game/Maps/Level1_Spiritual.Level1_Spiritual"))

(event `self.ReceiveBeginPlay`)

(event `Open Door`
  (bind _returnvalue (`SceneComponent.K2_GetComponentLocation` (`self.uwu`)))
  (bind (_direction _door_rotation) (`Timeline|Open Door Anim`)
    (:`Update`
      (`SceneComponent.K2_SetWorldLocation` (`self.uwu`) (`KismetMathLibrary.VLerp` _returnvalue (+ _returnvalue (0.0 0.0 -10.0)) _door_rotation) false false))))

(event `Collect Item`
  (`/Engine/EditorBlueprintResources/StandardMacros.IncrementInt` (`self.CurrentItemsCollected`)
    (:`  `
      (if (>= (`self.CurrentItemsCollected`) (`self.MaxItemsCollectable`))
        (`/Engine/EditorBlueprintResources/StandardMacros.DoOnce` false
          (:`Completed`
            (`KismetSystemLibrary.Delay` 2.0)
            (`self.Open Door`)))))))

(fn `UserConstructionScript`)